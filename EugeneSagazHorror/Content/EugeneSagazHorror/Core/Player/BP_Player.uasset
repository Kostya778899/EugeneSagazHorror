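; BP_Player is a first-person-style player character with axis-driven movement and look, hold-Left-Shift crouching and a camera shake started at BeginPlay.
; Movement follows control rotation.
; Each Tick plays or reverses the CameraCrouch timeline by crouch state, setting the camera scene component's world Z.
; That height lerps toward an absolute 50 from the cached start location's Y component, rather than its Z.
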(event `self.ReceiveBeginPlay`
  (`|ExecutionSequence`
    (:`then_0`
      (`CameraShakeSourceComponent.StartCameraShake` :`self` (`self.CameraShakeSource`) :`InCameraShake` "/Game/EugeneSagazHorror/Core/Player/Camera/BP_Camera_Shake.BP_Camera_Shake_C"))
    (:`then_1`
      (set `self.CameraSceneStartWorldLocation` (`SceneComponent.K2_GetComponentLocation` (`self.CameraScene`))))))

(event `self.ReceiveTick`
  (params (DeltaSeconds :type "Float (single-precision)"))
  (bind (_camerascenestartworldlocation_x _camerascenestartworldlocation_y) (`KismetMathLibrary.BreakVector` (`self.CameraSceneStartWorldLocation`)))
  (bind _camerascene (`self.CameraScene`))
  (bind (_returnvalue_x _returnvalue_y) (`KismetMathLibrary.BreakVector` (`SceneComponent.K2_GetComponentLocation` _camerascene)))
  (if (`self.bIsCrouched`)
    (bind (_direction _locationznormalized) (`Timeline|CameraCrouch` :!label _label)
      (:`Update`
        (`SceneComponent.K2_SetWorldLocation` _camerascene (`KismetMathLibrary.MakeVector` _returnvalue_x _returnvalue_y (`KismetMathLibrary.Lerp` _camerascenestartworldlocation_y 50.0 _locationznormalized)) false false)))
    (else
      (goto _label :!via `Reverse`))))

(event `InputAxis|MoveForward`
  (params (AxisValue :type "Float (single-precision)"))
  (`self.AddMovementInput` (`KismetMathLibrary.GetForwardVector` (`self.GetControlRotation`)) AxisValue true))

(event `InputAxis|MoveRight`
  (params (AxisValue :type "Float (single-precision)"))
  (`self.AddMovementInput` (`KismetMathLibrary.GetRightVector` (`self.GetControlRotation`)) AxisValue true))

(event `InputAxis|Turn`
  (params (AxisValue :type "Float (single-precision)"))
  (`self.AddControllerYawInput` AxisValue))

(event `InputAxis|LookUP`
  (params (AxisValue :type "Float (single-precision)"))
  (`self.AddControllerPitchInput` AxisValue))

(event `Key|LeftShift`
  (params (Key :type "Key Structure"))
  (:`Pressed`
    (`self.Crouch`))
  (:`Released`
    (`self.UnCrouch`)))

(event `self.K2_OnStartCrouch`
  (params (HalfHeightAdjust :type "Float (single-precision)") (ScaledHalfHeightAdjust :type "Float (single-precision)")))

(event `self.K2_OnEndCrouch`
  (params (HalfHeightAdjust :type "Float (single-precision)") (ScaledHalfHeightAdjust :type "Float (single-precision)")))

(fn `UserConstructionScript`)